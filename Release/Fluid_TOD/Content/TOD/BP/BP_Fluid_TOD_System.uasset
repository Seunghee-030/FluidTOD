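; Time-of-day sky system that orients sun and moon from start time and latitude and drives the sky dome and moon visuals.
; Construction sets the pivot rotations, creates dynamic materials for the dome and moon, and places the moon mesh along the moon's direction.
; OnUpdateCustomMaterials scrolls the sky UV offset and scales the moon by time or override.
; An optional debug widget, refreshed on Tick, shows clock, sunrise/sunset, intensities and day speed.
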(event EventBeginPlay
  ;[0.8371 0.06415 0.08 0.5] Evnet BeginPlay
  (CallFunction|InitDefault))

(event EventTick
  (params (DeltaSeconds :type Float%20%28single-precision%29))
  ;[0.9918 0.1554 0] Debug
  (CallFunction|DebugMode (Class|TODManager|GetCurrentTime)))

(event EventOnUpdateCustomMaterials
  (params (CurrentTime :type Float%20%28single-precision%29))
  ;[1 0.7711 0.1146] Sky/Moon Material Update
  (CallFunction|UpdateMaterial CurrentTime))

(fn ConstructionScript
  (bind _sun (Variables|Default|GetSun))
  ;[0.15 0.15 0.15 0.5] Init Sun&Moon Rotaion
  (Transformation|SetRelativeRotation (Variables|Default|GetPivotSunMoon) (Class|TODManager|CalculatePivotRotation (Variables|Default|GetStartTime)) false false)
  (Transformation|SetRelativeRotation (Variables|Default|GetPivotOrbitTilt) (Math|Rotator|MakeRotator (* (Variables|Default|Getlatitude) -1.0) 0.0 0.0) false false)
  (Transformation|SetRelativeRotation _sun "0, 0, 0" false false)
  (Transformation|SetRelativeRotation (Variables|Default|GetMoon) (Math|Rotator|MakeRotator 0.0 (+ (.pitch (Variables|/Script/Engine.SceneComponent|GetRelativeRotation _sun)) 1.8e+02) 0.0) false false)
  ;[1 0.7711 0.1146] Set Sky/Moon Materials
  (CallFunction|InitSkyMaterial)
  (CallFunction|InitMoon)
  (CallFunction|UpdateMaterial (Variables|Default|GetStartTime)))

(fn DebugMode
  (params (InTime :type Float%20%28double-precision%29))
  (bind _returnvalue (Class|TODManager|GetCurrentTime))
  (bind _debugwidget (Variables|DefaultSettings|GetDebugWidget))
  (bind _debugwidget_2 (Variables|DefaultSettings|GetDebugWidget))
  (if (Variables|Default|GetbEnableDebugPrint)
    (Widget|SetVisibility _debugwidget_2 "Visible")
    (Default|UpdateClockText _debugwidget (Utilities|Text|ToText(String) (Class|TODManager|GetFormattedTimeasString _returnvalue)))
    (Default|UpdateStaticTxt _debugwidget (Utilities|Text|ToText(Float) (Variables|Default|GetLatitude) "HalfToEven") (Utilities|Text|ToText(String) (Variables|Default|GetSunriseTime)) (Utilities|Text|ToText(String) (Variables|Default|GetSunsetTime)))
    (Default|UpdateSunIntensityText _debugwidget (Utilities|Text|ToText(Integer) (Math|Float|Truncate (Class|TODManager|GetSunIntensity _returnvalue))))
    (Default|UpdateMoonIntensity _debugwidget (Utilities|Text|ToText(Integer) (Math|Float|Truncate (Class|TODManager|GetMoonIntensity _returnvalue))))
    (Default|UpdateFinalDaySpeed _debugwidget (Utilities|Text|ToText(Float) (Class|TODManager|GetFinalSpeed _returnvalue) "HalfToEven"))
    (else
      (Widget|SetVisibility _debugwidget_2 "Hidden"))))

(fn InitDefault
  ;[0.15 0.15 0.15 0.5] Init PlayerRef
  (Variables|Default|SetPlayerRef (Game|GetPlayerCharacter 0))
  ;[0.15 0.15 0.15 0.5] Widget
  (bind _returnvalue (UserInterface|CreateWidget "/Fluid_TOD/TOD/Widget/WBP_DebugWidget.WBP_DebugWidget_C"))
  (UserInterface|Viewport|AddtoViewport _returnvalue 0)
  (Variables|DefaultSettings|SetDebugWidget _returnvalue))

(fn UpdateMaterial
  (params (InTime :type Float%20%28double-precision%29))
  (bind _returnvalue (Class|TODManager|GetMoonSourceScaleatTime InTime))
  (bind _overriddenmoonsourcescale (Variables|Default|GetOverriddenMoonSourceScale))
  (bind _skymaterialinstance (Variables|Default|GetSkyMaterialInstance))
  (bind _moonsourcemesh (Variables|Default|GetMoonSourceMesh))
  ;[0.1327 0.477 0.8547] Sky Dome Rotate
  (Utilities|IsValid _skymaterialinstance
    (:Is%20Valid
      (Rendering|Material|SetScalarParameterValue _skymaterialinstance "Sky UV Offset" (/ InTime 24.0) :!class /Script/Engine.MaterialInstanceDynamic))
    (:Is%20Not%20Valid
      _))
  ;[1 0.8705 0.3028] Moon Scale / Rotate
  (if (Variables|Default|GetbOverrideMoonSourceScale)
    (Transformation|SetWorldScale3D _moonsourcemesh (Math|Vector|MakeVector _overriddenmoonsourcescale _overriddenmoonsourcescale _overriddenmoonsourcescale))
    (else
      (Transformation|SetWorldScale3D _moonsourcemesh (Math|Vector|MakeVector _returnvalue _returnvalue _returnvalue)))))

(fn InitMoon
  ;[0.15 0.15 0.15 0.5] Material Settings
  (bind _returnvalue (Rendering|Material|CreateDynamicMaterialInstance (Variables|Default|GetMoonSourceMesh) 0 "/Fluid_TOD/TOD/Materials/MI_Moon.MI_Moon" "None" :!class /Script/Engine.PrimitiveComponent))
  (bind _output_get (Variables|Default|SetMoonMaterialInstance _returnvalue))
  (Utilities|IsValid _output_get
    (:Is%20Valid
      (Rendering|Material|SetTextureParameterValue (Variables|Default|GetMoonMaterialInstance) "MoonTexture_Base" (Variables|TOD|Texture|GetMoon%20Texture))
      (Rendering|Material|SetVectorParameterValue (Variables|Default|GetMoonMaterialInstance) "MoonEmissiveColor" (Variables|TOD|Texture|GetMoon%20Emissive%20Color) :!class /Script/Engine.MaterialInstanceDynamic))
    (:Is%20Not%20Valid
      _))
  ;[0.15 0.15 0.15 0.5] Mesh Rotation, Location Settings
  (Transformation|SetWorldRotation (Variables|Default|GetMoonSourceMesh) (Math|Rotator|MakeRotfromXZ (Math|Vector|GetForwardVector (Variables|Default|GetMoon)) (Variables|Etc|GetZ)) false false)
  (Transformation|SetWorldLocation (Variables|Default|GetMoonSourceMesh) (* (Math|Vector|Normalize (Math|Vector|GetForwardVector (Variables|Default|GetMoon))) (* (Variables|Etc|GetMoon%20Distance) -1.0)) false false))

(fn InitSkyMaterial
  (bind _returnvalue (Rendering|Material|CreateDynamicMaterialInstance (Variables|Default|GetSkydome) 0 "/Fluid_TOD/TOD/Materials/MI_Sky.MI_Sky" "None" :!class /Script/Engine.PrimitiveComponent))
  (bind _output_get (Variables|Default|SetSkyMaterialInstance _returnvalue))
  (Utilities|IsValid _output_get
    (:Is%20Valid
      (Rendering|Material|SetTextureParameterValue (Variables|Default|GetSkyMaterialInstance) "SkyDome Texture" (Variables|TOD|Texture|GetSky%20Dome%20Texture))
      (Rendering|Material|SetVectorParameterValue (Variables|Default|GetSkyMaterialInstance) "SkyTextureEmissiveColor" (Variables|TOD|Texture|GetSky%20Texture%20Tint) :!class /Script/Engine.MaterialInstanceDynamic))))