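; BP_Moon is a moon actor that keeps itself turned toward the player at a configurable uniform scale.
; Each Tick points its X axis from its location to the player pawn and reapplies Scale.
; The Construction Script does the same toward Origin, previewing orientation and size in the editor.
; BeginPlay caches the Player pawn, though Tick fetches it again directly.
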(event EventBeginPlay
  (Variables|Default|SetPlayer (Game|Player|GetPlayerPawn 0)))

(event Collision|EventActorBeginOverlap
  (params (OtherActor :type Actor%20Object%20Reference)))

(event EventTick
  (params (DeltaSeconds :type Float%20%28single-precision%29))
  (Transformation|SetActorRotation (Math|Conversions|RotationFromXVector (Math|Vector|Normalize (- (Transformation|GetActorLocation (Game|Player|GetPlayerPawn 0)) (Transformation|GetActorLocation)))))
  (Transformation|SetActorScale3D (Math|Conversions|ToVector(Float) (Variables|Default|GetScale))))

(fn ConstructionScript
  (Transformation|SetActorRotation (Math|Conversions|RotationFromXVector (Math|Vector|Normalize (- (Variables|Default|GetOrigin) (Transformation|GetActorLocation)))))
  (Transformation|SetActorScale3D (Math|Conversions|ToVector(Float) (Variables|Default|GetScale))))