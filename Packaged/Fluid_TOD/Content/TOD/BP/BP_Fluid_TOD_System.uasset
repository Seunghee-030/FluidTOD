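; Time-of-day Blueprint that drives the skydome's appearance and an on-screen debug readout.
; The construction script creates a dynamic sky material with configurable sky, star, moon and glow settings, then applies the start time.
; OnUpdateCustomMaterials scrolls the sky UV offset by the time as a fraction of 24 hours.
; BeginPlay creates the debug widget, and Tick refreshes its clock, sun, moon, speed and state readouts or hides it per EnableDebugPrint.
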(event EventBeginPlay
  ;[0.8371 0.06415 0.08 0.5] Evnet BeginPlay
  (CallFunction|InitDefault))

(event EventTick
  (params (DeltaSeconds :type Float%20%28single-precision%29))
  ;[0.9918 0.1554 0] Debug
  (CallFunction|DebugMode (Class|TODManager|GetCurrentTime)))

(event EventOnUpdateCustomMaterials
  (params (CurrentTime :type Float%20%28single-precision%29))
  ;[1 0.7711 0.1146] Sky/Moon Material Update
  (CallFunction|UpdateMaterial CurrentTime))

(fn ConstructionScript
  ;[1 0.7711 0.1146] Set Sky/Moon Materials
  (CallFunction|InitSkyMaterial)
  (CallFunction|UpdateMaterial (Variables|Default|GetStartTime)))

(fn DebugMode
  (params (InTime :type Float%20%28double-precision%29))
  (bind _returnvalue (Class|TODManager|GetCurrentTime))
  (bind _debugwidget (Variables|DefaultSettings|GetDebugWidget))
  (bind _debugwidget_2 (Variables|DefaultSettings|GetDebugWidget))
  (if (Variables|Default|GetbEnableDebugPrint)
    (Widget|SetVisibility _debugwidget_2 "Visible")
    (Default|UpdateClockText _debugwidget (Utilities|Text|ToText(String) (Class|TODManager|GetFormattedTimeasString _returnvalue)))
    (Default|UpdateStaticTxt _debugwidget (Utilities|Text|ToText(Float) (Variables|Default|GetLatitude) "HalfToEven") (Utilities|Text|ToText(String) (Variables|Default|GetSunriseTime)) (Utilities|Text|ToText(String) (Variables|Default|GetSunsetTime)))
    (Default|UpdateSunIntensityText _debugwidget (Utilities|Text|ToText(Integer) (Math|Float|Truncate (Class|TODManager|GetSunIntensity _returnvalue))))
    (Default|UpdateMoonIntensity _debugwidget (Utilities|Text|ToText(Integer) (Math|Float|Truncate (Class|TODManager|GetMoonIntensity _returnvalue))))
    (Default|UpdateFinalDaySpeed _debugwidget (Utilities|Text|ToText(Float) (Class|TODManager|GetFinalSpeed _returnvalue) "HalfToEven"))
    (Default|UpdateStateText _debugwidget (Utilities|Text|ToText(String) (Utilities|String|EnumtoString (Class|TODManager|GetCurrentTODState (Class|TODManager|GetCurrentTime)))))
    (else
      (Widget|SetVisibility _debugwidget_2 "Hidden"))))

(fn InitDefault
  ;[0.15 0.15 0.15 0.5] Init PlayerRef
  (Variables|Default|SetPlayerRef (Game|GetPlayerCharacter 0))
  ;[0.15 0.15 0.15 0.5] Widget
  (bind _returnvalue (UserInterface|CreateWidget "/Fluid_TOD/TOD/Widget/WBP_DebugWidget.WBP_DebugWidget_C"))
  (UserInterface|Viewport|AddtoViewport _returnvalue 0)
  (Variables|DefaultSettings|SetDebugWidget _returnvalue))

(fn UpdateMaterial
  (params (InTime :type Float%20%28double-precision%29))
  (bind _skymaterialinstance (Variables|Default|GetSkyMaterialInstance))
  ;[0.1327 0.477 0.8547] Sky Dome Rotate
  (Utilities|IsValid _skymaterialinstance
    (:Is%20Valid
      (Rendering|Material|SetScalarParameterValue _skymaterialinstance "Sky UV Offset" (/ InTime 24.0) :!class /Script/Engine.MaterialInstanceDynamic))))

(fn InitSkyMaterial
  (bind _returnvalue (Rendering|Material|CreateDynamicMaterialInstance (Variables|Default|GetSkydome) 0 "/Fluid_TOD/TOD/Materials/MI_Sky.MI_Sky" "None" :!class /Script/Engine.PrimitiveComponent))
  (bind _output_get (Variables|Default|SetSkyMaterialInstance _returnvalue))
  (Utilities|IsValid _output_get
    (:Is%20Valid
      (Rendering|Material|SetTextureParameterValue (Variables|Default|GetSkyMaterialInstance) "SkyDome Texture" (Variables|TOD|Texture|GetSky%20Dome%20Texture))
      (Rendering|Material|SetTextureParameterValue (Variables|Default|GetSkyMaterialInstance) "Star Mask Texture" (Variables|TOD|Texture|GetStar%20Mask%20Texture))
      (Rendering|Material|SetScalarParameterValue (Variables|Default|GetSkyMaterialInstance) "UseStarMask" (Math|Conversions|ToFloat(Boolean) (Variables|TOD|Texture|GetUse%20Star%20Mask%20Texture)) :!class /Script/Engine.MaterialInstanceDynamic)
      (Rendering|Material|SetVectorParameterValue (Variables|Default|GetSkyMaterialInstance) "SkyTextureEmissiveColor" (Variables|TOD|Texture|GetSky%20Texture%20Tint) :!class /Script/Engine.MaterialInstanceDynamic)
      (Rendering|Material|SetVectorParameterValue (Variables|Default|GetSkyMaterialInstance) "StarEmissiveColor" (Variables|TOD|Texture|GetStar%20Texture%20Tint) :!class /Script/Engine.MaterialInstanceDynamic)
      (Rendering|Material|SetTextureParameterValue (Variables|Default|GetSkyMaterialInstance) "MoonTexture" (Variables|TOD|Texture|GetMoon%20Texture))
      (Rendering|Material|SetVectorParameterValue (Variables|Default|GetSkyMaterialInstance) "MoonEmissiveColor" (Variables|TOD|Texture|GetMoon%20Emissive%20Color) :!class /Script/Engine.MaterialInstanceDynamic)
      (Rendering|Material|SetScalarParameterValue (Variables|Default|GetSkyMaterialInstance) "MoonRotation" (Variables|TOD|Texture|GetMoon%20Rotation) :!class /Script/Engine.MaterialInstanceDynamic)
      (Rendering|Material|SetTextureParameterValue (Variables|Default|GetSkyMaterialInstance) "MoonGlowTexture" (Variables|TOD|Texture|GetMoon%20Glow%20Texture))
      (Rendering|Material|SetVectorParameterValue (Variables|Default|GetSkyMaterialInstance) "MoonGlowEmissiveColor" (Variables|TOD|Texture|GetMoon%20Glow%20Emissive%20Color) :!class /Script/Engine.MaterialInstanceDynamic))))